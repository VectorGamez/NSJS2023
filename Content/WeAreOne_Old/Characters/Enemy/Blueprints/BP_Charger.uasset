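; BP_Charger is an enemy character that targets players it sees and deals melee damage.
; PawnSensing on authority writes any seen pawn with a health component to the blackboard Target key.
; PrepareAttack tints a dynamic material red as a telegraph; Attack clears it and damages the first player in a sphere overlap.
; GetParried launches it backwards and briefly stops its AI logic before restarting it.
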(event `self.PawnSensing.OnSeePawn`
  (params (Pawn :type "Pawn Object Reference"))
  (`/Engine/EditorBlueprintResources/ActorMacros.Switch Has Authority`
    (:`Authority`
      (`/Engine/EditorBlueprintResources/StandardMacros.IsValid` (`/Game/WeAreOne_Old/Gameplay/BP_HelperLibrary.GetHealthComponent` Pawn)
        (:`Is Valid`
          (`BlackboardComponent.SetValueAsObject` (`AIBlueprintHelperLibrary.GetBlackboard` null) "Target" Pawn))))))

(event `self.GetParried`
  (bind _braincomponent (`AIController.BrainComponent` (`AIBlueprintHelperLibrary.GetAIController` self)))
  (`self.LaunchCharacter` (* (`self.GetActorForwardVector`) -1500) true)
  (`BrainComponent.StopLogic` _braincomponent "")
  (`KismetSystemLibrary.Delay` 2.0)
  (`BrainComponent.RestartLogic` _braincomponent))

(event `self.Attack`
  (params (ActorToAttack :type "Actor Object Reference"))
  (`self.PrepareAttack` false)
  (bind (_outactors _returnvalue) (`KismetSystemLibrary.SphereOverlapActors` (`self.K2_GetActorLocation`) (`self.AttackRange`) (`|MakeArray` "ObjectTypeQuery3" :!type "EObjectTypeQuery Enum") "/Game/WeAreOne_Old/Characters/Player/Blueprints/BP_Character_Player.BP_Character_Player_C"))
  (if _returnvalue
    (`/Game/WeAreOne_Old/Gameplay/BP_Health_Component.TakeDamage` (`/Game/WeAreOne_Old/Gameplay/BP_HelperLibrary.GetHealthComponent` (`|GetArrayItem` _outactors)) (`self.Damage`) self)))

(event `PrepareAttack`
  (params (Prepared :type Boolean))
  (`/Engine/EditorBlueprintResources/StandardMacros.Can Execute Cosmetic Events`
    (:`True`
      (`MaterialInstanceDynamic.SetVectorParameterValue` (`self.MID`) "Color" (`KismetMathLibrary.SelectColor` (struct :`R` 1.0 :`A` 1.0) (struct :`R` 1.0 :`G` 1.0 :`B` 1.0 :`A` 1.0) Prepared)))))

(fn `UserConstructionScript`
  (bind _returnvalue (`PrimitiveComponent.CreateDynamicMaterialInstance` (`self.Sphere`) 0 null "None"))
  (set `self.MID` _returnvalue))