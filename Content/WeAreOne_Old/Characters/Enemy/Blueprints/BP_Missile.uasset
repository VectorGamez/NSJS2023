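; Enemy missile pawn that starts AI-controlled, then turns into a physics-driven projectile that damages what it hits.
; While possessed, pawn sensing writes any seen pawn with a health component to the blackboard as Target.
; Turntomissile unpossesses it, enables gravity-free capsule physics, attaches a Niagara trail and sets a lifespan; Tick then accelerates it forward below a speed cap.
; Impacts apply damage to health components and destroy it, as does being parried.
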(event `self.ReceiveTick`
  (params (DeltaSeconds :type "Float (single-precision)"))
  (bind _capsulecomponent (`self.CapsuleComponent`))
  (`parent.ReceiveTick` DeltaSeconds)
  (if (`self.IsMissle`)
    (if (<= (`KismetMathLibrary.VSize` (`SceneComponent.GetComponentVelocity` _capsulecomponent)) (`self.MaxMissileSpeed`))
      (`PrimitiveComponent.AddForce` _capsulecomponent (* (`self.GetActorForwardVector`) 5000.0) "None" true))))

(event `Turn to missile`
  (bind _capsulecomponent (`self.CapsuleComponent`))
  (set `self.IsMissle` true)
  (`Controller.UnPossess` (`AIBlueprintHelperLibrary.GetAIController` self))
  (`CapsuleComponent.SetCapsuleHalfHeight` _capsulecomponent 40.0 true)
  (`PrimitiveComponent.SetSimulatePhysics` _capsulecomponent true)
  (`PrimitiveComponent.SetEnableGravity` _capsulecomponent false)
  (`NiagaraFunctionLibrary.SpawnSystemAttached` "/Game/WeAreOne_Old/Gameplay/PlayerProjectile/NS_BulletTrail.NS_BulletTrail" (`self.CapsuleComponent`) "None" (-60.0 0.0 0.0) (struct) "KeepRelativeOffset" true)
  (`self.SetLifeSpan` 5.0))

(event `self.PawnSensing.OnSeePawn`
  (params (Pawn :type "Pawn Object Reference"))
  (`/Engine/EditorBlueprintResources/StandardMacros.IsValid` (`/Game/WeAreOne_Old/Gameplay/BP_HelperLibrary.GetHealthComponent` Pawn)
    (:`Is Valid`
      (`BlackboardComponent.SetValueAsObject` (`AIBlueprintHelperLibrary.GetBlackboard` null) "Target" Pawn))))

(event `self.CapsuleComponent.OnComponentHit`
  (params (HitComponent :type "PrimitiveComponent Object Reference") (OtherActor :type "Actor Object Reference") (OtherComp :type "PrimitiveComponent Object Reference") (NormalImpulse :type "Vector Structure") (Hit :type "HitResult Structure (by ref)"))
  (bind _return (`/Game/WeAreOne_Old/Gameplay/BP_HelperLibrary.GetHealthComponent` OtherActor))
  (if (`self.IsMissle`)
    (`/Engine/EditorBlueprintResources/StandardMacros.IsValid` _return
      (:`Is Valid`
        (`/Game/WeAreOne_Old/Gameplay/BP_Health_Component.TakeDamage` _return (`self.Damage`) self))
      (:`Is Not Valid`
        _))
    (`self.K2_DestroyActor`)))

(event `self.GetParried`
  (`self.K2_DestroyActor`))

(event `Rotate`
  (params (delta :type "Rotator Structure"))
  (`SceneComponent.K2_SetRelativeRotation` (`self.Mesh`) delta false false))

(fn `UserConstructionScript`)