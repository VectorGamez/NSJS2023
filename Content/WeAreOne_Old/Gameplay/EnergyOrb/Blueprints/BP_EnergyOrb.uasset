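; BP_EnergyOrb is a pickup that heals player characters who touch it, using its EnergyAmount value.
; On BeginPlay the authority launches the sphere with a velocity-change impulse, random sideways and upward at MaxForce, so it pops out.
; On overlap the authority casts to BP_Character_Player, calls Heal on that character's health component and destroys the orb.
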(event `self.ReceiveBeginPlay`
  (bind _maxforce (`self.MaxForce`))
  (bind _returnvalue (* _maxforce -1.0))
  (`/Engine/EditorBlueprintResources/ActorMacros.Switch Has Authority`
    (:`Authority`
      (`PrimitiveComponent.AddImpulse` (`self.Sphere1`) (`KismetMathLibrary.MakeVector` (`KismetMathLibrary.RandomFloatInRange` _returnvalue _maxforce) (`KismetMathLibrary.RandomFloatInRange` _returnvalue _maxforce) _maxforce) "None" true))))

(event `self.ReceiveActorBeginOverlap`
  (params (OtherActor :type "Actor Object Reference"))
  (`/Engine/EditorBlueprintResources/ActorMacros.Switch Has Authority`
    (:`Authority`
      (bind _asbp_character_player (cast `/Game/WeAreOne_Old/Characters/Player/Blueprints/BP_Character_Player` OtherActor))
      (`/Game/WeAreOne_Old/Gameplay/BP_Health_Component.Heal` (`/Game/WeAreOne_Old/Gameplay/BP_HelperLibrary.GetHealthComponent` _asbp_character_player) (`self.EnergyAmount`))
      (`self.K2_DestroyActor`))))

(fn `UserConstructionScript`)