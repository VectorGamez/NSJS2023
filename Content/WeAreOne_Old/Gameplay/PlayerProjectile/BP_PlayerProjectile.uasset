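; Player-fired projectile that explodes on impact, damaging enemies and knocking them back.
; Any component hit destroys it, first applying contact damage through the health component if it struck a BP_Enemy_Base.
; Destruction spawns explosion VFX and sound where cosmetics can run.
; On authority only, it also sphere-overlaps nearby enemies, applying explosion damage and launching characters outward with added upward force.
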(event `self.Collision.OnComponentHit`
  (params (HitComponent :type "PrimitiveComponent Object Reference") (OtherActor :type "Actor Object Reference") (OtherComp :type "PrimitiveComponent Object Reference") (NormalImpulse :type "Vector Structure") (Hit :type "HitResult Structure (by ref)"))
  (`/Engine/EditorBlueprintResources/StandardMacros.IsValid` (`/Game/WeAreOne_Old/Gameplay/BP_HelperLibrary.GetHealthComponent` OtherActor)
    (:`Is Valid`
      (cast `/Game/WeAreOne_Old/Characters/Enemy/Blueprints/BP_Enemy_Base` OtherActor
        (:`then`
          (`/Game/WeAreOne_Old/Gameplay/BP_Health_Component.TakeDamage` (`/Game/WeAreOne_Old/Gameplay/BP_HelperLibrary.GetHealthComponent` OtherActor) (`self.ContactDamage`) self)
          (`self.K2_DestroyActor`))
        (:`CastFailed`
          (`self.K2_DestroyActor` :!label _label))))
    (:`Is Not Valid`
      (goto _label))))

(event `self.ReceiveDestroyed`
  (bind _returnvalue (`self.K2_GetActorLocation`))
  (`/Engine/EditorBlueprintResources/StandardMacros.Can Execute Cosmetic Events`
    (:`True`
      (`NiagaraFunctionLibrary.SpawnSystemAtLocation` "/Game/WeAreOne_Old/Shared/VFX/NS_Explosion_Projectile.NS_Explosion_Projectile" (`self.K2_GetActorLocation`))
      (bind _returnvalue_2 (`GameplayStatics.SpawnSoundAtLocation` "/Game/WeAreOne_Old/Shared/Sounds/SC_Explosion.SC_Explosion" _returnvalue (struct) 1.0 1.0 0.0 null null))
      (`AudioComponent.FadeIn` _returnvalue_2 2.0 1.0 0.0 "Linear"))
    (:`False`
      _))
  (`/Engine/EditorBlueprintResources/ActorMacros.Switch Has Authority`
    (:`Authority`
      (bind _outactors (`KismetSystemLibrary.SphereOverlapActors` _returnvalue (`self.AOERange`) (`|MakeArray` "ObjectTypeQuery3" :!type "EObjectTypeQuery Enum") "/Game/WeAreOne_Old/Characters/Enemy/Blueprints/BP_Enemy_Base.BP_Enemy_Base_C"))
      (for _array_element _outactors
        (`/Engine/EditorBlueprintResources/StandardMacros.IsValid` _array_element
          (:`Is Valid`
            (bind _ascharacter (cast `Character` _array_element))
            (`/Game/WeAreOne_Old/Gameplay/BP_Health_Component.TakeDamage` (`/Game/WeAreOne_Old/Gameplay/BP_HelperLibrary.GetHealthComponent` _ascharacter) (`self.ExplosionDamage`) null)
            (`/Engine/EditorBlueprintResources/StandardMacros.IsValid` _ascharacter
              (:`Is Valid`
                (`Character.LaunchCharacter` _ascharacter (+ (* (`KismetMathLibrary.GetDirectionUnitVector` (`self.K2_GetActorLocation`) (`self.K2_GetActorLocation` _array_element)) (`self.KnockbackMagnitude`)) (`KismetMathLibrary.MakeVector` 0.0 0.0 (`self.UpwardForce`))) true true)))))))))

(fn `UserConstructionScript`)