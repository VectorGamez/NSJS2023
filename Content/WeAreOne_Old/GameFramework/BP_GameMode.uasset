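; Game mode that spawns the player character at a PlayerStart and assigns control for single-player or two-player sessions.
; PostLogin reads the MultiPlayer option and runs setup once enough players register, waiting for two on a dedicated multiplayer server.
; Player 1 possesses the character; Player 2, created locally unless on a dedicated server, possesses its helper pawn.
; Each gets an input mapping context, and single-player adds extra bindings to Player 1.
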(event `self.K2_PostLogin`
  (params (NewPlayer :type "PlayerController Object Reference"))
  (bind _returnvalue (`GameplayStatics.GetPlayerController` 1))
  (`/Engine/EditorBlueprintResources/StandardMacros.Gate` false :!label _label
    (:`Exit`
      (set `self.IsMultiPlayer` (`GameplayStatics.HasOption` (`self.OptionsString`) "MultiPlayer"))
      (bind _allregistered (`self.RegisterPlayer` NewPlayer))
      (if _allregistered
        (`|ExecutionSequence`
          (:`then_0`
            (goto _label :!via `Close`))
          (:`then_1`
            (`|ExecutionSequence`
              (:`then_0`
                ;[1 1 1] Spawn and initialize Player 1
                (bind _asbp_player_controller (cast `/Game/WeAreOne_Old/Characters/Player/Blueprints/BP_PlayerController` (`GameplayStatics.GetPlayerController` 0)))
                (`/Game/WeAreOne_Old/Characters/Player/Blueprints/BP_PlayerController.OwningClient_AddMappingContext` _asbp_player_controller "/Game/WeAreOne_Old/Input/MappingContexts/IMC_Player1.IMC_Player1")
                (bind _returnvalue_2 (`|SpawnActorFromClass` "/Game/WeAreOne_Old/Characters/Player/Blueprints/BP_Character_Player.BP_Character_Player_C" (`self.GetStartTransform`) "AlwaysSpawn" "MultiplyWithRoot" null null))
                (bind _output_get (set `self.CharacterPlayer` _returnvalue_2))
                (`Controller.Possess` (`GameplayStatics.GetPlayerController` 0) _output_get))
              (:`then_1`
                (if (`self.IsMultiPlayer`)
                  (if (not (`KismetSystemLibrary.IsDedicatedServer`))
                    ;[1 1 1] Initialize Player 2
                    (`GameplayStatics.CreatePlayer` -1))
                  (bind _asbp_player_controller_2 (cast `/Game/WeAreOne_Old/Characters/Player/Blueprints/BP_PlayerController` _returnvalue))
                  (`/Game/WeAreOne_Old/Characters/Player/Blueprints/BP_PlayerController.OwningClient_AddMappingContext` _asbp_player_controller_2 "/Game/WeAreOne_Old/Input/MappingContexts/IMC_Player2.IMC_Player2")
                  (`Controller.Possess` _returnvalue (`/Game/WeAreOne_Old/Characters/Player/Blueprints/BP_Character_Player.GetHelperPawn` (`self.CharacterPlayer`)))
                  (else
                    ;[1 1 1] Add single player additional key bindings for player 1
                    (bind _asbp_player_controller_3 (cast `/Game/WeAreOne_Old/Characters/Player/Blueprints/BP_PlayerController` (`GameplayStatics.GetPlayerController` 0)))
                    (`/Game/WeAreOne_Old/Characters/Player/Blueprints/BP_PlayerController.OwningClient_AddMappingContext` _asbp_player_controller_3 "/Game/WeAreOne_Old/Input/MappingContexts/IMC_SinglePlayer_Additional.IMC_SinglePlayer_Additional")))))))))))

(fn `GetStartTransform`
  (returns (StartTransform :type "Transform Structure (by ref)"))
  (locals (PlayerStart :type "PlayerStart Object Reference"))
  (bind _returnvalue (`GameplayStatics.GetActorOfClass` "/Script/Engine.PlayerStart"))
  (bind _output_get (set `local.PlayerStart` _returnvalue))
  (`/Engine/EditorBlueprintResources/StandardMacros.IsValid` _output_get
    (:`Is Valid`
      (return (`self.GetTransform` _output_get)))))

(fn `RegisterPlayer`
  (params (Player :type "PlayerController Object Reference (by ref)"))
  (returns (AllRegistered :type Boolean))
  (bind _returnvalue (`KismetArrayLibrary.Array_AddUnique` (`self.Player`) Player))
  (return (>= _returnvalue (and (`self.IsMultiPlayer`) (`KismetSystemLibrary.IsDedicatedServer`)))))

(fn `UserConstructionScript`)