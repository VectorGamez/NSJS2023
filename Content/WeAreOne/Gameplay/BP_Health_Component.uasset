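; Health component that tracks current health for its owner and broadcasts damage and death.
; Health starts at MaxHealth on BeginPlay.
; TakeDamage only acts while health is above zero, firing OnDamaged with damage and instigator, then zeroing health and firing OnDeath when depleted.
; Heal adds an amount clamped between zero and MaxHealth, with no check for death.
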(event `self.ReceiveBeginPlay`
  (set `self.Health` (`self.Max Health`)))

(event `TakeDamage`
  (params (Damage :type "Float (double-precision)") (Instigator :type "Actor Object Reference"))
  (bind _health (`self.Health`))
  (if (> _health 0.0)
    (bind _output_get (set `self.Health` (- _health Damage)))
    (`self.OnDamaged` Damage Instigator)
    (if (<= _output_get 0.0)
      (set `self.Health` 0.0)
      (`self.OnDeath`))))

(event `Heal`
  (params (Amount :type "Float (double-precision)"))
  (set `self.Health` (`KismetMathLibrary.FClamp` (+ Amount (`self.Health`)) 0.0 (`self.Max Health`))))