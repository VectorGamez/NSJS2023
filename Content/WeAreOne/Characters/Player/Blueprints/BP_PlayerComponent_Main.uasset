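; BP_PlayerComponent_Main is a player component that turns tagged input into movement for BP_Player_Character_Main.
; On BeginPlay it casts its owner to that character and caches the reference.
; NativeInputTagTriggered switches on the gameplay tag, and Input.Move feeds the action value's X and Y into AddMovementInput along the actor's right and forward vectors.
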(event `self.ReceiveBeginPlay`
  (bind _asbp_player_character_main (cast `/Game/WeAreOne/Characters/Player/Blueprints/BP_Player_Character_Main` (`self.GetOwner`)))
  (set `self.Player` _asbp_player_character_main))

(event `self.ReceiveNativeInputTagTriggered`
  (params (input_tag :type "GameplayTag Structure") (input_action_value :type "InputActionValue Structure (by ref)"))
  (bind (_x _y) (`EnhancedInputLibrary.BreakInputActionValue` input_action_value))
  (bind _player (`self.Player`))
  (`|SwitchGameplayTag` input_tag
    (:`Input.Move`
      (`Pawn.AddMovementInput` _player (+ (* _x (`Actor.GetActorRightVector` _player)) (* _y (`Actor.GetActorForwardVector` _player))) 1.0 false))))