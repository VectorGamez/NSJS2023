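; Player component for the helper pawn that handles its rotation input.
; On BeginPlay it caches the owning BP_Player_Pawn_Helper.
; The Input.Rotate tag turns the 2D axis into a world direction, using the main player's camera right and forward vectors flattened to 2D.
; It then snaps the helper to face that direction, giving camera-relative aiming.
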(event `self.ReceiveBeginPlay`
  (bind _asbp_player_pawn_helper (cast `/Game/WeAreOne/Characters/Player/Blueprints/BP_Player_Pawn_Helper` (`self.GetOwner`)))
  (set `self.Helper` _asbp_player_pawn_helper))

(event `self.ReceiveNativeInputTagTriggered`
  (params (input_tag :type "GameplayTag Structure") (input_action_value :type "InputActionValue Structure (by ref)"))
  (`|SwitchGameplayTag` input_tag
    (:`Input.Rotate`
      (`self.Rotate` input_action_value))))

(event `Rotate`
  (params (InputActionValue :type "InputActionValue Structure"))
  (bind (_x _y) (`EnhancedInputLibrary.BreakInputActionValue` InputActionValue))
  (bind _camera (`/Game/WeAreOne/Characters/Player/Blueprints/BP_Player_Character_Main.Camera` (`/Game/WeAreOne/Characters/Player/Blueprints/BP_Player_Pawn_Helper.GetPlayerMain` (`self.Helper`))))
  (`Actor.K2_SetActorRotation` (`self.Helper`) (`KismetMathLibrary.Conv_VectorToRotator` (`KismetMathLibrary.Normal` (+ (* _x (`KismetMathLibrary.Vector_Normal2D` (`SceneComponent.GetRightVector` _camera))) (* _y (`KismetMathLibrary.Vector_Normal2D` (`SceneComponent.GetForwardVector` _camera)))))) false))