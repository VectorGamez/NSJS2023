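; Player helper actor that acts as an aimable cannon for its owning player, adding the player HUD locally on initialization.
; Aim input sets a camera-relative direction, which a box-trace aim assist snaps toward actors with health components as Tick smooths rotation.
; Shooting is gated by reload time and multicasts cosmetics, while authority spawns the projectile, knocks the owner back and consumes energy.
; A line trace sizes the laser pointer each Tick.
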(event `Initialize`
  (params (PlayerOwner :type "/Game/WeAreOne/Characters/Player/Blueprints/BP_Character_Player Object Reference"))
  (bind _output_get (set `self.PlayerOwner` PlayerOwner))
  (`SceneComponent.K2_AttachToComponent` (`self.Camera`) (`/Game/WeAreOne/Characters/Player/Blueprints/BP_Character_Player.Camera` _output_get) "None" "SnapToTarget" "SnapToTarget" "KeepWorld" true)
  (if (`self.IsLocallyControlled`)
    (bind _returnvalue (`|CreateWidget` "/Game/WeAreOne/Characters/Player/UI/WBP_Player.WBP_Player_C" (`GameplayStatics.GetPlayerController` 0) (`/Game/WeAreOne/Characters/Player/Blueprints/BP_Character_Player.BP_Health_Component` _output_get)))
    (`UserWidget.AddToViewport` _returnvalue 0)))

(event `EnhancedInput|/Game/WeAreOne/Input/Actions/IA_Shoot`
  (params (ActionValue :type Boolean) (ElapsedSeconds :type "Float (double-precision)") (TriggeredSeconds :type "Float (double-precision)") (InputAction :type "InputAction Object Reference" :default "/Game/WeAreOne/Input/Actions/IA_Shoot.IA_Shoot"))
  (:`Triggered`
    (`self.Shoot`)))

(event `multicastShoot`
  (`|ExecutionSequence`
    (:`then_0`
      (`/Engine/EditorBlueprintResources/StandardMacros.Can Execute Cosmetic Events`
        (:`True`
          (`AudioComponent.Play` (`self.SC_CannonShot`) 0.0)
          (`MaterialInstanceDynamic.SetVectorParameterValue` (`self.MID`) "Color" (struct :`R` 1.0 :`G` 0.573 :`A` 1.0))
          (`PlayerCameraManager.StartCameraShake` :`self` (`GameplayStatics.GetPlayerCameraManager` 0) :`ShakeClass` "/Game/WeAreOne/Characters/Player/VFX/BP_Shoot_Shake.BP_Shoot_Shake_C" :`Scale` 8.0)
          (`ActorComponent.Activate` (`self.NS_MuzzleFlash`) true)
          (`MaterialInstanceDynamic.SetVectorParameterValue` (`self.MID`) "Color" (struct :`R` 1.0 :`A` 1.0))
          (`MaterialInstanceDynamic.SetVectorParameterValue` (`self.MID`) "Color" (struct :`G` 1.0 :`A` 1.0)))))
    (:`then_1`
      (`/Engine/EditorBlueprintResources/ActorMacros.Switch Has Authority`
        (:`Authority`
          (`CharacterMovementComponent.AddImpulse` (`Character.CharacterMovement` (`self.PlayerOwner`)) (+ (* (* (`self.GetActorForwardVector`) -1.0) (`self.KnockbackMagnitude`)) (`KismetMathLibrary.MakeVector` 0.0 0.0 (`self.UpwardForce`))) true)
          (`|SpawnActorFromClass` "/Game/WeAreOne/Gameplay/PlayerProjectile/BP_PlayerProjectile.BP_PlayerProjectile_C" (`SceneComponent.K2_GetComponentToWorld` (`self.Arrow`)) "AlwaysSpawn" "MultiplyWithRoot" self null)
          (`/Game/WeAreOne/Characters/Player/Blueprints/BP_Character_Player.ConsumeEnergy` (`self.PlayerOwner`) (`self.ShotEnergy`)))))))

(event `EnhancedInput|/Game/WeAreOne/Input/Actions/IA_Aim`
  (params (ActionValue :type "Vector2D Structure") (ElapsedSeconds :type "Float (double-precision)") (TriggeredSeconds :type "Float (double-precision)") (InputAction :type "InputAction Object Reference" :default "/Game/WeAreOne/Input/Actions/IA_Aim.IA_Aim"))
  (:`Triggered`
    (`self.Aim` ActionValue)))

(event `Shoot`
  (`/Engine/EditorBlueprintResources/StandardMacros.DoOnce` false :!label _label
    (:`Completed`
      (`self.multicastShoot`)
      (`KismetSystemLibrary.Delay` (`self.ReloadTime`))
      (goto _label :!via `Reset`))))

(event `Aim`
  (params (ActionValue :type "Vector2D Structure"))
  (bind (_x _y) (`KismetMathLibrary.BreakVector2D` ActionValue))
  (bind _playerowner (`self.PlayerOwner`)
    (:`then`
      (bind _camera (`/Game/WeAreOne/Characters/Player/Blueprints/BP_Character_Player.Camera` _playerowner))
      (set `self.DesiredLookDirection` (`KismetMathLibrary.Vector_Normal2D` (+ (* (`SceneComponent.GetRightVector` _camera) _x) (* (`KismetMathLibrary.Vector_Normal2D` (`SceneComponent.GetForwardVector` _camera)) _y)))))
    (:`else`)))

(event `self.ReceiveBeginPlay`
  (set `self.DesiredLookDirection` (`SceneComponent.GetForwardVector` (`self.Arrow`))))

(event `self.ReceiveTick`
  (params (DeltaSeconds :type "Float (single-precision)"))
  (bind _laserpointerdistance (`self.LaserPointerDistance`))
  (bind _cylinder (`self.Cylinder`))
  (bind _arrow (`self.Arrow`))
  (bind _returnvalue (`SceneComponent.K2_GetComponentLocation` _arrow))
  (bind (_returnvalue_x _returnvalue_y) (`KismetMathLibrary.BreakVector` (`SceneComponent.K2_GetComponentScale` _cylinder)))
  (`|ExecutionSequence`
    (:`then_0`
      (bind _desiredrotation (`self.CalculateAimAssist`))
      (`self.K2_SetActorRotation` (`KismetMathLibrary.RLerp` (`self.K2_GetActorRotation`) _desiredrotation 0.5 true)))
    (:`then_1`
      (bind (_outhit _returnvalue_2) (`KismetSystemLibrary.LineTraceSingle` _returnvalue (+ _returnvalue (* (`SceneComponent.GetForwardVector` _arrow) (`self.LaserPointerDistance`))) "TraceTypeQuery1"))
      (bind (_bblockinghit _binitialoverlap _time _distance) (`GameplayStatics.BreakHitResult` _outhit))
      (`SceneComponent.SetWorldScale3D` _cylinder (`KismetMathLibrary.MakeVector` _returnvalue_x _returnvalue_y (`KismetMathLibrary.SelectFloat` (/ _distance 100.0) (/ _laserpointerdistance 100.0) _returnvalue_2)))
      (bind _returnvalue_3 (`KismetMathLibrary.SelectFloat` _distance _laserpointerdistance _returnvalue_2))
      (`SceneComponent.K2_SetRelativeLocation` _cylinder (`KismetMathLibrary.MakeVector` (* _returnvalue_3 0.5)) false false)
      (`SceneComponent.K2_SetRelativeLocation` (`self.Sphere`) (`KismetMathLibrary.MakeVector` _returnvalue_3) false false))))

(fn `CalculateAimAssist`
  (returns (DesiredRotation :type "Rotator Structure"))
  (bind _desiredlookdirection (`self.DesiredLookDirection`))
  (bind _outhits (`KismetSystemLibrary.BoxTraceMulti` (+ (`self.K2_GetActorLocation`) (* _desiredlookdirection (`self.AimAssistMinDistance`))) (+ (`SceneComponent.K2_GetComponentLocation` (`self.Arrow`)) (* _desiredlookdirection (`self.AimAssistDistance`))) (`self.AimAssistSize`) (struct) "TraceTypeQuery1"))
  (bind (_location _distance _found) (`self.GetTargetForAimAssist` _outhits))
  (return (`KismetMathLibrary.SelectRotator` (`KismetMathLibrary.FindLookAtRotation` (`self.K2_GetActorLocation`) _location) (`KismetMathLibrary.Conv_VectorToRotator` (`self.DesiredLookDirection`)) _found)))

(fn `GetTargetForAimAssist`
  (params (Array :type "Array of HitResult Structure"))
  (returns (Location :type "Vector Structure") (Distance :type "Float (single-precision)") (Found :type Boolean))
  (for _array_element Array
    (bind (_bblockinghit _binitialoverlap _time _distance _location _impactpoint _normal _impactnormal _physmat _hitactor) (`GameplayStatics.BreakHitResult` _array_element))
    (`/Engine/EditorBlueprintResources/StandardMacros.IsValid` _hitactor
      (:`Is Valid`
        (`/Engine/EditorBlueprintResources/StandardMacros.IsValid` (`/Game/WeAreOne/Gameplay/BP_HelperLibrary.GetHealthComponent` _hitactor)
          (:`Is Valid`
            (return (`self.K2_GetActorLocation` _hitactor) _distance true))))))
  (return (0.0 0.0 0.0) 0.0 false))

(fn `UserConstructionScript`
  (bind _returnvalue (`PrimitiveComponent.CreateDynamicMaterialInstance` (`self.Cube`) 0 null "None"))
  (set `self.MID` _returnvalue))