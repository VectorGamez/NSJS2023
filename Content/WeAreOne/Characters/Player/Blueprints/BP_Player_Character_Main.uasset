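; Main player character Blueprint that owns a player helper pawn through a child actor component.
; On BeginPlay the authority makes itself the helper's owner, and a getter returns that child actor cast to BP_Player_Pawn_Helper.
; It also binds to the CharacterExtensionComponent's input setup delegate, which has the BP_PlayerController apply additional input mappings.
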(event `self.ReceiveBeginPlay`
  ;[1 1 1] :TODO: How can we remove this?
  (`/Engine/EditorBlueprintResources/ActorMacros.Switch Has Authority`
    (:`Authority`
      (`self.SetOwner` (`ChildActorComponent.ChildActor` (`self.Player_Helper`)) self))
    (:`Remote`
      _))
  (add `GFPawnExtensionComponent.OnSetupPlayerInputComponentDelegate` (`self.CharacterExtensionComponent`) (delegate `OnSetupPlayerInputComponent`)))

(event `OnSetupPlayerInputComponent`
  (params (input_component :type "InputComponent Object Reference"))
  ;[1 1 1] :TODO: How can we remove this?
  (bind _asbp_player_controller (cast `/Game/WeAreOne/Characters/Player/Blueprints/BP_PlayerController` (`self.GetController`)))
  (`/Game/WeAreOne/Characters/Player/Blueprints/BP_PlayerController.ApplyAdditionalInputMappings` _asbp_player_controller))

(fn `GetPlayerHelper`
  (returns (PlayerHelper :type "/Game/WeAreOne/Characters/Player/Blueprints/BP_Player_Pawn_Helper Object Reference"))
  (bind _asbp_player_pawn_helper (cast `/Game/WeAreOne/Characters/Player/Blueprints/BP_Player_Pawn_Helper` (`ChildActorComponent.ChildActor` (`self.Player_Helper`))))
  (return _asbp_player_pawn_helper))

(fn `UserConstructionScript`)