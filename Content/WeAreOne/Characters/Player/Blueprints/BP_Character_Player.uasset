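; Player character that spends health as energy when moving or jumping and handles shielding, death and the HUD, pause and end screens.
; Shooting and aiming route to a child-actor player helper.
; The shield refunds part of incoming damage, while an early-timed block refunds it fully and parries enemies around the attacker.
; Death starts an explosion countdown timeline that cancels if health recovers, with cosmetic and authority logic gated separately.
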(event `self.ReceiveBeginPlay`
  (bind _asbp_player_helper (cast `/Game/WeAreOne/Characters/Player/Blueprints/BP_Player_Helper` (`ChildActorComponent.ChildActor` (`self.Helper`))))
  (bind _output_get (set `self.PlayerHelper` _asbp_player_helper))
  (`/Game/WeAreOne/Characters/Player/Blueprints/BP_Player_Helper.Initialize` _output_get self)
  (`/Engine/EditorBlueprintResources/StandardMacros.Can Execute Cosmetic Events`
    (:`True`
      (bind _returnvalue (`|CreateWidget` "/Game/WeAreOne/Characters/Player/UI/WBP_Player.WBP_Player_C" (`GameplayStatics.GetPlayerController` 0) (`/Game/WeAreOne/Gameplay/BP_HelperLibrary.GetHealthComponent` self)))
      (`UserWidget.AddToViewport` _returnvalue 0))))

(event `EnhancedInput|/Game/WeAreOne/Input/Actions/IA_Move`
  (params (ActionValue :type "Vector2D Structure") (ElapsedSeconds :type "Float (double-precision)") (TriggeredSeconds :type "Float (double-precision)") (InputAction :type "InputAction Object Reference" :default "/Game/WeAreOne/Input/Actions/IA_Move.IA_Move"))
  (bind (_x _y) (`KismetMathLibrary.BreakVector2D` ActionValue))
  (bind _camera (`self.Camera`))
  (:`Triggered`
    (`self.AddMovementInput` (+ (* (`SceneComponent.GetRightVector` _camera) _x) (* (`KismetMathLibrary.Vector_Normal2D` (`SceneComponent.GetForwardVector` _camera)) _y)))
    (`self.ConsumeEnergy` (* (`self.MovementEnergy`) (`GameplayStatics.GetWorldDeltaSeconds`)))))

(event `EnhancedInput|/Game/WeAreOne/Input/Actions/IA_Jump`
  (params (ActionValue :type Boolean) (ElapsedSeconds :type "Float (double-precision)") (TriggeredSeconds :type "Float (double-precision)") (InputAction :type "InputAction Object Reference" :default "/Game/WeAreOne/Input/Actions/IA_Jump.IA_Jump"))
  (:`Triggered`
    (`self.Jump`)
    (if (`self.CanJump`)
      (`self.ConsumeEnergy` (`self.JumpEnergy`)))))

(event `EnhancedInput|/Game/WeAreOne/Input/Actions/IA_Shield`
  (params (ActionValue :type Boolean) (ElapsedSeconds :type "Float (double-precision)") (TriggeredSeconds :type "Float (double-precision)") (InputAction :type "InputAction Object Reference" :default "/Game/WeAreOne/Input/Actions/IA_Shield.IA_Shield"))
  (bind _sphere (`self.Sphere`))
  (:`Triggered`
    (set `self.ShieldActiveTime` TriggeredSeconds))
  (:`Started`
    (`SceneComponent.SetHiddenInGame` _sphere false false)
    (set `self.ShieldActive` true))
  (:`Canceled`
    (`SceneComponent.SetHiddenInGame` _sphere true false :!label _label)
    (set `self.ShieldActive` false))
  (:`Completed`
    (goto _label)))

(event `EnhancedInput|/Game/WeAreOne/Input/Actions/IA_Shoot`
  (params (ActionValue :type Boolean) (ElapsedSeconds :type "Float (double-precision)") (TriggeredSeconds :type "Float (double-precision)") (InputAction :type "InputAction Object Reference" :default "/Game/WeAreOne/Input/Actions/IA_Shoot.IA_Shoot"))
  ;[1 0 0.2175] SinglePlayer Routing
  (:`Triggered`
    (`/Game/WeAreOne/Characters/Player/Blueprints/BP_Player_Helper.Shoot` (`self.PlayerHelper`))))

(event `EnhancedInput|/Game/WeAreOne/Input/Actions/IA_Aim`
  (params (ActionValue :type "Vector2D Structure") (ElapsedSeconds :type "Float (double-precision)") (TriggeredSeconds :type "Float (double-precision)") (InputAction :type "InputAction Object Reference" :default "/Game/WeAreOne/Input/Actions/IA_Aim.IA_Aim"))
  ;[1 0 0.2175] SinglePlayer Routing
  (:`Triggered`
    (`/Game/WeAreOne/Characters/Player/Blueprints/BP_Player_Helper.Aim` (`self.PlayerHelper`) ActionValue)))

(event `self.BP_Health_Component.OnDamaged`
  (params (Damage :type "Float (double-precision)") (Instigator :type "Actor Object Reference"))
  (bind _bp_health_component (`self.BP_Health_Component`))
  (`|ExecutionSequence`
    (:`then_0`
      (if (and (not (`self.ShieldActive`)) (> Damage 0.0) (`.bSuccess` (cast `/Game/WeAreOne/Characters/Enemy/Blueprints/BP_Enemy_Base` Instigator :!pure true)))
        (`self.PlayDamagedParticle`)))
    (:`then_1`
      (if (and (> Damage 0.0) (`self.ShieldActive`) (!= Instigator self))
        (if (<= (`self.ShieldActiveTime`) 0.5)
          (`/Game/WeAreOne/Gameplay/BP_Health_Component.Heal` _bp_health_component (* Damage 1.0))
          (bind _outactors (`KismetSystemLibrary.SphereOverlapActors` (`self.K2_GetActorLocation` Instigator) (`self.ParryRadius`) (`|MakeArray` "ObjectTypeQuery3" :!type "EObjectTypeQuery Enum") "/Game/WeAreOne/Characters/Enemy/Blueprints/BP_Enemy_Base.BP_Enemy_Base_C"))
          (for _array_element _outactors
            (bind _asbp_enemy_base (cast `/Game/WeAreOne/Characters/Enemy/Blueprints/BP_Enemy_Base` _array_element))
            (`/Game/WeAreOne/Characters/Enemy/Blueprints/BP_Enemy_Base.GetParried` _asbp_enemy_base))
          (else
            (`/Game/WeAreOne/Gameplay/BP_Health_Component.Heal` _bp_health_component (* Damage 0.5))))))))

(event `self.BP_Health_Component.OnDeath`
  (`/Engine/EditorBlueprintResources/StandardMacros.Can Execute Cosmetic Events`
    (:`True`
      (bind _returnvalue (`NiagaraFunctionLibrary.SpawnSystemAttached` "/Game/WeAreOne/Shared/VFX/NS_Explosion_Loop.NS_Explosion_Loop" (`self.CapsuleComponent`) "None" (0.0 0.0 0.0) (struct) "KeepRelativeOffset" true))
      (set `self.AboutToExplodeFX` _returnvalue))
    (:`False`
      _))
  (`/Engine/EditorBlueprintResources/ActorMacros.Switch Has Authority`
    (:`Authority`
      (`TimelineComponent.PlayFromStart` (`self.AboutToExplode`)))))

(event `PlayDamagedParticle`
  (`NiagaraFunctionLibrary.SpawnSystemAtLocation` "/Game/WeAreOne/Shared/VFX/NS_Damaged.NS_Damaged" (`self.K2_GetActorLocation`)))

(event `OnDie`
  (bind _charactermovement (`self.CharacterMovement`))
  (`|ExecutionSequence`
    (:`then_0`
      (`/Engine/EditorBlueprintResources/StandardMacros.Can Execute Cosmetic Events`
        (:`True`
          (`NiagaraFunctionLibrary.SpawnSystemAtLocation` "/Game/WeAreOne/Shared/VFX/NS_Explosion.NS_Explosion" (`self.K2_GetActorLocation`))
          (`self.DisableInput` null)
          (`PlayerCameraManager.StartCameraFade` :`self` (`GameplayStatics.GetPlayerCameraManager` 0) :`ToAlpha` 1.0 :`Duration` 3.0 :`bShouldFadeAudio` true :`bHoldWhenFinished` true)
          (`WidgetLayoutLibrary.RemoveAllWidgets`)
          (bind _returnvalue (`|CreateWidget` "/Game/WeAreOne/Characters/Player/UI/WBP_EndScreen.WBP_EndScreen_C" (cast `PlayerController` (`self.GetController`) :!pure true)))
          (`UserWidget.AddToViewport` _returnvalue 0))))
    (:`then_1`
      (`self.SetActorHiddenInGame` true))
    (:`then_2`
      (`/Engine/EditorBlueprintResources/ActorMacros.Switch Has Authority`
        (:`Authority`
          (`MovementComponent.StopMovementImmediately` _charactermovement)
          (`CharacterMovementComponent.SetMovementMode` _charactermovement "MOVE_Flying" 0))))))

(event `EnhancedInput|/Game/WeAreOne/Input/Actions/IA_Escape`
  (params (ActionValue :type Boolean) (ElapsedSeconds :type "Float (double-precision)") (TriggeredSeconds :type "Float (double-precision)") (InputAction :type "InputAction Object Reference" :default "/Game/WeAreOne/Input/Actions/IA_Escape.IA_Escape"))
  (:`Triggered`
    (bind _returnvalue (`|CreateWidget` "/Game/WeAreOne/Characters/Player/UI/WBP_Pause.WBP_Pause_C" (cast `PlayerController` (`self.GetController`) :!pure true)))
    (`UserWidget.AddToViewport` _returnvalue 0)
    (`GameplayStatics.SetGamePaused` true)))

(fn `ConsumeEnergy`
  (params (Energy :type "Float (double-precision)"))
  (`/Game/WeAreOne/Gameplay/BP_Health_Component.TakeDamage` (`self.BP_Health_Component`) Energy self))

(fn `GetHelperPawn`
  (returns (HelperPawn :type "Pawn Object Reference"))
  (bind _aspawn (cast `Pawn` (`ChildActorComponent.ChildActor` (`self.Helper`))))
  (return _aspawn))

(fn `UserConstructionScript`)