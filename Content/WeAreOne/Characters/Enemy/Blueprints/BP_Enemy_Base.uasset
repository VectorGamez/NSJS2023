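; Base enemy actor with health, a world-space status widget, and empty GetParried and Attack events.
; On cosmetic-capable instances it passes its health component to WBP_Enemy and turns the widget toward the camera each tick.
; Damage spawns a Niagara hit effect and death destroys the actor.
; On destruction the authority spawns energy orbs around it, while cosmetic-capable instances play an explosion.
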(event `self.ReceiveTick`
  (params (DeltaSeconds :type "Float (single-precision)"))
  (`/Engine/EditorBlueprintResources/StandardMacros.Can Execute Cosmetic Events`
    (:`True`
      (`SceneComponent.K2_SetWorldRotation` (`self.Widget`) (`KismetMathLibrary.FindLookAtRotation` (`self.K2_GetActorLocation`) (`PlayerCameraManager.GetCameraLocation` (`GameplayStatics.GetPlayerCameraManager` 0))) false false))))

(event `self.ReceiveBeginPlay`
  (`/Engine/EditorBlueprintResources/StandardMacros.Can Execute Cosmetic Events`
    (:`True`
      (bind _aswbp_enemy (cast `/Game/WeAreOne/Characters/Enemy/UI/WBP_Enemy` (`WidgetComponent.GetWidget` (`self.Widget`))))
      (set `/Game/WeAreOne/Characters/Enemy/UI/WBP_Enemy.HealthComponent` (`self.BP_Health_Component`) _aswbp_enemy))))

(event `GetParried`)

(event `Attack`
  (params (ActorToAttack :type "Actor Object Reference")))

(event `self.ReceiveDestroyed`
  (`|ExecutionSequence`
    (:`then_0`
      (`/Engine/EditorBlueprintResources/ActorMacros.Switch Has Authority`
        (:`Authority`
          (for _ (range 1 (+ (`self.EnergyOrbAmount`) 1))
            (`|SpawnActorFromClass` "/Game/WeAreOne/Gameplay/EnergyOrb/Blueprints/BP_EnergyOrb.BP_EnergyOrb_C" (`KismetMathLibrary.MakeTransform` (`KismetMathLibrary.RandomPointInBoundingBox` (+ (`self.K2_GetActorLocation`) (0.0 0.0 100.0)) (15.0 15.0 15.0))) "AlwaysSpawn" "MultiplyWithRoot" null null)))))
    (:`then_1`
      (`/Engine/EditorBlueprintResources/StandardMacros.Can Execute Cosmetic Events`
        (:`True`
          (`NiagaraFunctionLibrary.SpawnSystemAtLocation` "/Game/WeAreOne/Shared/VFX/NS_Explosion.NS_Explosion" (`self.K2_GetActorLocation`)))))))

(event `self.BP_Health_Component.OnDeath`
  (`self.K2_DestroyActor`))

(event `self.BP_Health_Component.OnDamaged`
  (params (Damage :type "Float (double-precision)") (Instigator :type "Actor Object Reference"))
  (`NiagaraFunctionLibrary.SpawnSystemAtLocation` "/Game/WeAreOne/Shared/VFX/NS_Damaged.NS_Damaged" (`self.K2_GetActorLocation`)))

(fn `UserConstructionScript`)