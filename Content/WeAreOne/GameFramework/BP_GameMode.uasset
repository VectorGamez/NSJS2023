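; Game mode that spawns and possesses the shared player character for single-player or two-player play.
; PostLogin records joining controllers and runs setup once a newly added one has index 1 or higher.
; The first controller receives an input config and possesses a character spawned at a PlayerStart.
; The "Singleplayer" option gives it the additional mapping context; otherwise the second controller gets that context and possesses the character's helper pawn.
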(event `self.K2_PostLogin`
  (params (NewPlayer :type "PlayerController Object Reference"))
  (bind _returnvalue (`GameplayStatics.GetPlayerController` 1))
  (bind _returnvalue_2 (`GameplayStatics.GetPlayerController` 0))
  (bind _returnvalue_3 (`KismetArrayLibrary.Array_AddUnique` (`self.Player`) NewPlayer))
  (if (>= _returnvalue_3 1)
    (set `self.IsSinglePlayer` (`GameplayStatics.HasOption` (`self.OptionsString`) "Singleplayer"))
    (`|ExecutionSequence`
      (:`then_0`
        (bind _asbp_player_controller (cast `/Game/WeAreOne/Characters/Player/Blueprints/BP_PlayerController` _returnvalue_2))
        (`/Game/WeAreOne/Characters/Player/Blueprints/BP_PlayerController.OwningClient_AddMappableConfig` _asbp_player_controller "/Game/WeAreOne/Input/InputConfigs/PMIC_Player1.PMIC_Player1")
        (bind _returnvalue_4 (`GameplayStatics.GetActorOfClass` "/Script/Engine.PlayerStart"))
        (`/Engine/EditorBlueprintResources/StandardMacros.IsValid` _returnvalue_4
          (:`Is Valid`
            (bind _returnvalue_5 (`|SpawnActorFromClass` "/Game/WeAreOne/Characters/Player/Blueprints/BP_Character_Player.BP_Character_Player_C" (`self.GetTransform` _returnvalue_4) "AlwaysSpawn" "MultiplyWithRoot" null null))
            (bind _output_get (set `self.PlayerCharacter` _returnvalue_5))
            (`Controller.Possess` (`GameplayStatics.GetPlayerController` 0) _output_get))))
      (:`then_1`
        (if (`self.IsSinglePlayer`)
          (bind _asbp_player_controller_2 (cast `/Game/WeAreOne/Characters/Player/Blueprints/BP_PlayerController` _returnvalue_2))
          (`/Game/WeAreOne/Characters/Player/Blueprints/BP_PlayerController.OwningClient_AddMappingContext` _asbp_player_controller_2 "/Game/WeAreOne/Input/MappingContexts/IMC_SinglePlayer_Additional.IMC_SinglePlayer_Additional")
          (else
            (bind _asbp_player_controller_3 (cast `/Game/WeAreOne/Characters/Player/Blueprints/BP_PlayerController` _returnvalue))
            (`/Game/WeAreOne/Characters/Player/Blueprints/BP_PlayerController.OwningClient_AddMappingContext` _asbp_player_controller_3 "/Game/WeAreOne/Input/MappingContexts/IMC_SinglePlayer_Additional.IMC_SinglePlayer_Additional")
            (`Controller.Possess` _returnvalue (`/Game/WeAreOne/Characters/Player/Blueprints/BP_Character_Player.GetHelperPawn` (`self.PlayerCharacter`)))))))))

(fn `UserConstructionScript`)