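; BP_Player_Helper is the player's aimable shooter actor, firing projectiles and knocking its owner backward and upward.
; Camera-relative aim input sets a look direction, which a box trace overrides toward the first hit actor with a health component.
; Tick eases rotation toward that result and fits a laser pointer to a line trace.
; A DoOnce and delay gate reloading, shown by red and green material color.
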(event `Initialize`
  (params (PlayerOwner :type "/Game/NSJS2023/Characters/Player/Blueprints/BP_Character_Player Object Reference"))
  (set `self.PlayerOwner` PlayerOwner))

(event `EnhancedInput|/Game/NSJS2023/Input/Actions/IA_Shoot`
  (params (ActionValue :type Boolean) (ElapsedSeconds :type "Float (double-precision)") (TriggeredSeconds :type "Float (double-precision)") (InputAction :type "InputAction Object Reference" :default "/Game/NSJS2023/Input/Actions/IA_Shoot.IA_Shoot"))
  (:`Triggered`
    (if (`NavMovementComponent.IsMovingOnGround` (`Character.CharacterMovement` (`self.PlayerOwner`)))
      _
      (else
        _))
    (`/Engine/EditorBlueprintResources/StandardMacros.DoOnce` false :!label _label
      (:`Completed`
        (`CharacterMovementComponent.AddImpulse` (`Character.CharacterMovement` (`self.PlayerOwner`)) (+ (* (* (`self.GetActorForwardVector`) -1.0) (`self.KnockbackMagnitude`)) (`KismetMathLibrary.MakeVector` 0.0 0.0 (`self.UpwardForce`))) true)
        (`|SpawnActorFromClass` "/Game/NSJS2023/Gameplay/PlayerProjectile/BP_PlayerProjectile.BP_PlayerProjectile_C" (`SceneComponent.K2_GetComponentToWorld` (`self.Arrow`)) "AlwaysSpawn" "MultiplyWithRoot" null null)
        (`MaterialInstanceDynamic.SetVectorParameterValue` (`self.MID`) "Color" (struct :`R` 1.0 :`A` 1.0))
        (`KismetSystemLibrary.Delay` (`self.ReloadTime`))
        (`MaterialInstanceDynamic.SetVectorParameterValue` (`self.MID`) "Color" (struct :`G` 1.0 :`A` 1.0))
        (goto _label :!via `Reset`)))))

(event `EnhancedInput|/Game/NSJS2023/Input/Actions/IA_Aim`
  (params (ActionValue :type "Vector2D Structure") (ElapsedSeconds :type "Float (double-precision)") (TriggeredSeconds :type "Float (double-precision)") (InputAction :type "InputAction Object Reference" :default "/Game/NSJS2023/Input/Actions/IA_Aim.IA_Aim"))
  (bind (_x _y) (`KismetMathLibrary.BreakVector2D` ActionValue))
  (:`Triggered`
    (bind _playerowner (`self.PlayerOwner`)
      (:`then`
        (bind _camera (`/Game/NSJS2023/Characters/Player/Blueprints/BP_Character_Player.Camera` _playerowner))
        (set `self.DesiredLookDirection` (`KismetMathLibrary.Vector_Normal2D` (+ (* (`SceneComponent.GetRightVector` _camera) _x) (* (`KismetMathLibrary.Vector_Normal2D` (`SceneComponent.GetForwardVector` _camera)) _y)))))
      (:`else`))))

(event `self.ReceiveBeginPlay`
  (set `self.DesiredLookDirection` (`SceneComponent.GetForwardVector` (`self.Arrow`))))

(event `self.ReceiveTick`
  (params (DeltaSeconds :type "Float (single-precision)"))
  (bind _laserpointerdistance (`self.LaserPointerDistance`))
  (bind _cylinder (`self.Cylinder`))
  (bind _arrow (`self.Arrow`))
  (bind _returnvalue (`SceneComponent.K2_GetComponentLocation` _arrow))
  (bind (_returnvalue_x _returnvalue_y) (`KismetMathLibrary.BreakVector` (`SceneComponent.K2_GetComponentScale` _cylinder)))
  (`|ExecutionSequence`
    (:`then_0`
      (bind _desiredrotation (`self.CalculateAimAssist`))
      (`self.K2_SetActorRotation` (`KismetMathLibrary.RLerp` (`self.K2_GetActorRotation`) _desiredrotation 0.5 true)))
    (:`then_1`
      (bind (_outhit _returnvalue_2) (`KismetSystemLibrary.LineTraceSingle` _returnvalue (+ _returnvalue (* (`SceneComponent.GetForwardVector` _arrow) (`self.LaserPointerDistance`))) "TraceTypeQuery1"))
      (bind (_bblockinghit _binitialoverlap _time _distance) (`GameplayStatics.BreakHitResult` _outhit))
      (`SceneComponent.SetWorldScale3D` _cylinder (`KismetMathLibrary.MakeVector` _returnvalue_x _returnvalue_y (`KismetMathLibrary.SelectFloat` (/ _distance 100.0) (/ _laserpointerdistance 100.0) _returnvalue_2)))
      (bind _returnvalue_3 (`KismetMathLibrary.SelectFloat` _distance _laserpointerdistance _returnvalue_2))
      (`SceneComponent.K2_SetRelativeLocation` _cylinder (`KismetMathLibrary.MakeVector` (* _returnvalue_3 0.5)) false false)
      (`SceneComponent.K2_SetRelativeLocation` (`self.Sphere`) (`KismetMathLibrary.MakeVector` _returnvalue_3) false false))))

(fn `CalculateAimAssist`
  (returns (DesiredRotation :type "Rotator Structure"))
  (bind _desiredlookdirection (`self.DesiredLookDirection`))
  (bind _outhits (`KismetSystemLibrary.BoxTraceMulti` (+ (`self.K2_GetActorLocation`) (* _desiredlookdirection (`self.AimAssistMinDistance`))) (+ (`SceneComponent.K2_GetComponentLocation` (`self.Arrow`)) (* _desiredlookdirection (`self.AimAssistDistance`))) (`self.AimAssistSize`) (struct) "TraceTypeQuery1"))
  (bind (_location _distance _found) (`self.GetTargetForAimAssist` _outhits))
  (return (`KismetMathLibrary.SelectRotator` (`KismetMathLibrary.FindLookAtRotation` (`self.K2_GetActorLocation`) _location) (`KismetMathLibrary.Conv_VectorToRotator` (`self.DesiredLookDirection`)) _found)))

(fn `GetTargetForAimAssist`
  (params (Array :type "Array of HitResult Structure"))
  (returns (Location :type "Vector Structure") (Distance :type "Float (single-precision)") (Found :type Boolean))
  (for _array_element Array
    (bind (_bblockinghit _binitialoverlap _time _distance _location _impactpoint _normal _impactnormal _physmat _hitactor) (`GameplayStatics.BreakHitResult` _array_element))
    (`/Engine/EditorBlueprintResources/StandardMacros.IsValid` _hitactor
      (:`Is Valid`
        (`/Engine/EditorBlueprintResources/StandardMacros.IsValid` (`/Game/NSJS2023/Gameplay/BP_HelperLibrary.GetHealthComponent` _hitactor)
          (:`Is Valid`
            (return (`self.K2_GetActorLocation` _hitactor) _distance true))))))
  (return (0.0 0.0 0.0) 0.0 false))

(fn `UserConstructionScript`
  (bind _returnvalue (`PrimitiveComponent.CreateDynamicMaterialInstance` (`self.Cube`) 0 null "None"))
  (set `self.MID` _returnvalue))