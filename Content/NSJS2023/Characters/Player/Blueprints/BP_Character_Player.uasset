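; Player character Blueprint that handles camera-relative movement, jumping, HUD setup and a child-actor helper.
; On BeginPlay it initializes the BP_Player_Helper child actor with itself, then creates the WBP_Player widget bound to its health component.
; Enhanced Input drives movement along the camera's right and horizontally flattened forward vectors, plus jumping.
; GetHelperPawn exposes the helper child actor as a Pawn.
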(event `self.ReceiveBeginPlay`
  (bind _asbp_player_helper (cast `/Game/NSJS2023/Characters/Player/Blueprints/BP_Player_Helper` (`ChildActorComponent.ChildActor` (`self.Helper`))))
  (`/Game/NSJS2023/Characters/Player/Blueprints/BP_Player_Helper.Initialize` _asbp_player_helper self)
  (bind _returnvalue (`|CreateWidget` "/Game/NSJS2023/Characters/Player/UI/WBP_Player.WBP_Player_C" (`GameplayStatics.GetPlayerController` 0) (`/Game/NSJS2023/Gameplay/BP_HelperLibrary.GetHealthComponent` self)))
  (`UserWidget.AddToViewport` _returnvalue 0))

(event `EnhancedInput|/Game/NSJS2023/Input/Actions/IA_Move`
  (params (ActionValue :type "Vector2D Structure") (ElapsedSeconds :type "Float (double-precision)") (TriggeredSeconds :type "Float (double-precision)") (InputAction :type "InputAction Object Reference" :default "/Game/NSJS2023/Input/Actions/IA_Move.IA_Move"))
  (bind (_x _y) (`KismetMathLibrary.BreakVector2D` ActionValue))
  (bind _camera (`self.Camera`))
  (:`Triggered`
    (`self.AddMovementInput` (+ (* (`SceneComponent.GetRightVector` _camera) _x) (* (`KismetMathLibrary.Vector_Normal2D` (`SceneComponent.GetForwardVector` _camera)) _y)))))

(event `EnhancedInput|/Game/NSJS2023/Input/Actions/IA_Jump`
  (params (ActionValue :type Boolean) (ElapsedSeconds :type "Float (double-precision)") (TriggeredSeconds :type "Float (double-precision)") (InputAction :type "InputAction Object Reference" :default "/Game/NSJS2023/Input/Actions/IA_Jump.IA_Jump"))
  (:`Triggered`
    (`self.Jump`)))

(fn `GetHelperPawn`
  (returns (HelperPawn :type "Pawn Object Reference"))
  (bind _aspawn (cast `Pawn` (`ChildActorComponent.ChildActor` (`self.Helper`))))
  (return _aspawn))

(fn `UserConstructionScript`)