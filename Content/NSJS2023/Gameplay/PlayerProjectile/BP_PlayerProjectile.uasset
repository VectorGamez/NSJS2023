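; BP_PlayerProjectile is the player's projectile, dealing damage to actors that have a health component.
; On each Sphere hit it looks up the other actor's health component and applies Damage.
; A HitActors list limits damage to once per actor, and the projectile is not destroyed by these hits.
; Hitting anything without a valid health component destroys the projectile.
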(event `self.Sphere.OnComponentHit`
  (params (HitComponent :type "PrimitiveComponent Object Reference") (OtherActor :type "Actor Object Reference") (OtherComp :type "PrimitiveComponent Object Reference") (NormalImpulse :type "Vector Structure") (Hit :type "HitResult Structure (by ref)"))
  (`/Engine/EditorBlueprintResources/StandardMacros.IsValid` (`/Game/NSJS2023/Gameplay/BP_HelperLibrary.GetHealthComponent` OtherActor)
    (:`Is Valid`
      (if (not (`KismetArrayLibrary.Array_Contains` (`self.HitActors`) OtherActor))
        (`/Game/NSJS2023/Gameplay/BP_Health_Component.TakeDamage` (`/Game/NSJS2023/Gameplay/BP_HelperLibrary.GetHealthComponent` OtherActor) (`self.Damage`))
        (`KismetArrayLibrary.Array_Add` (`self.HitActors`) OtherActor)))
    (:`Is Not Valid`
      (`self.K2_DestroyActor`))))

(fn `UserConstructionScript`)