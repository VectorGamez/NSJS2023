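; Game mode that sets up the player character and input for either single-player or local two-player play.
; On BeginPlay it spawns BP_Character_Player at a PlayerStart, possesses it with controller 0 and applies that player's Enhanced Input config.
; IsSinglePlayer either adds an extra mapping context for player one, or creates a second local player with its own config that possesses the character's helper pawn.
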(event `self.ReceiveBeginPlay`
  (bind _returnvalue (`GameplayStatics.GetPlayerController` 1))
  (bind _returnvalue_2 (pcsubsystem `EnhancedInputLocalPlayerSubsystem` (`GameplayStatics.GetPlayerController` 0)))
  (`|ExecutionSequence`
    (:`then_0`
      (`EnhancedInputSubsystemInterface.AddPlayerMappableConfig` _returnvalue_2 "/Game/NSJS2023/Input/InputConfigs/PMIC_Player1.PMIC_Player1" (struct))
      (bind _returnvalue_3 (`GameplayStatics.GetActorOfClass` "/Script/Engine.PlayerStart"))
      (`/Engine/EditorBlueprintResources/StandardMacros.IsValid` _returnvalue_3
        (:`Is Valid`
          (bind _returnvalue_4 (`|SpawnActorFromClass` "/Game/NSJS2023/Characters/Player/Blueprints/BP_Character_Player.BP_Character_Player_C" (`self.GetTransform` _returnvalue_3) "Undefined" "MultiplyWithRoot" null null))
          (bind _output_get (set `self.PlayerCharacter` _returnvalue_4))
          (`Controller.Possess` (`GameplayStatics.GetPlayerController` 0) _output_get))))
    (:`then_1`
      (if (`self.IsSinglePlayer`)
        (`EnhancedInputSubsystemInterface.AddMappingContext` _returnvalue_2 "/Game/NSJS2023/Input/MappingContexts/IMC_SinglePlayer_Additional.IMC_SinglePlayer_Additional" 0 (struct))
        (else
          (`GameplayStatics.CreatePlayer` 1)
          (`EnhancedInputSubsystemInterface.AddPlayerMappableConfig` (pcsubsystem `EnhancedInputLocalPlayerSubsystem` _returnvalue) "/Game/NSJS2023/Input/InputConfigs/PMIC_Player2.PMIC_Player2" (struct))
          (`Controller.Possess` _returnvalue (`/Game/NSJS2023/Characters/Player/Blueprints/BP_Character_Player.GetHelperPawn` (`self.PlayerCharacter`))))))))

(fn `UserConstructionScript`)