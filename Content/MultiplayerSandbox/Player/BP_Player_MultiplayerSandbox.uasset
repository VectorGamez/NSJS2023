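; Player pawn for the multiplayer sandbox that moves, looks, shoots projectiles and dies when its health runs out.
; On BeginPlay it fills health, adds its Enhanced Input mapping context and puts a health widget on the viewport.
; Input drives camera-relative movement and controller look, while Shoot spawns a projectile from an arrow component with the player as owner.
; TakeDamage subtracts health and destroys the actor at zero or below.
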(event `self.ReceiveBeginPlay`
  (`|ExecutionSequence`
    (:`then_0`
      (set `self.Health` (`self.MaxHealth`)))
    (:`then_1`
      (bind _asplayer_controller (cast `PlayerController` (`self.GetController`)))
      (`EnhancedInputSubsystemInterface.AddMappingContext` (pcsubsystem `EnhancedInputLocalPlayerSubsystem` _asplayer_controller) "/Game/MultiplayerSandbox/Player/IMC_MultiplayerSandbox.IMC_MultiplayerSandbox" 0 (struct)))
    (:`then_2`
      (bind _returnvalue (`|CreateWidget` "/Game/MultiplayerSandbox/Player/WBP_MultiplayerSandbox_PlayerHealth.WBP_MultiplayerSandbox_PlayerHealth_C" (cast `PlayerController` (`self.GetController`) :!pure true)))
      (`UserWidget.AddToViewport` _returnvalue 0))))

(event `EnhancedInput|/Game/MultiplayerSandbox/Player/IA_MultiplayerSandbox_Move`
  (params (ActionValue :type "Vector2D Structure") (ElapsedSeconds :type "Float (double-precision)") (TriggeredSeconds :type "Float (double-precision)") (InputAction :type "InputAction Object Reference" :default "/Game/MultiplayerSandbox/Player/IA_MultiplayerSandbox_Move.IA_MultiplayerSandbox_Move"))
  (bind (_x _y) (`KismetMathLibrary.BreakVector2D` ActionValue))
  (bind _camera (`self.Camera`))
  (:`Triggered`
    (`self.AddMovementInput` (+ (* _x (`SceneComponent.GetRightVector` _camera)) (* _y (`SceneComponent.GetForwardVector` _camera))))))

(event `EnhancedInput|/Game/MultiplayerSandbox/Player/IA_MultiplayerSandbox_View`
  (params (ActionValue :type "Vector2D Structure") (ElapsedSeconds :type "Float (double-precision)") (TriggeredSeconds :type "Float (double-precision)") (InputAction :type "InputAction Object Reference" :default "/Game/MultiplayerSandbox/Player/IA_MultiplayerSandbox_View.IA_MultiplayerSandbox_View"))
  (bind (_x _y) (`KismetMathLibrary.BreakVector2D` ActionValue))
  (:`Triggered`
    (`self.AddControllerYawInput` _x)
    (`self.AddControllerPitchInput` (* _y -1.0))))

(event `EnhancedInput|/Game/MultiplayerSandbox/Player/IA_MultiplayerSandbox_Shoot`
  (params (ActionValue :type Boolean) (ElapsedSeconds :type "Float (double-precision)") (TriggeredSeconds :type "Float (double-precision)") (InputAction :type "InputAction Object Reference" :default "/Game/MultiplayerSandbox/Player/IA_MultiplayerSandbox_Shoot.IA_MultiplayerSandbox_Shoot"))
  (:`Triggered`
    (`self.Shoot`)))

(event `Shoot`
  (`|SpawnActorFromClass` "/Game/MultiplayerSandbox/Player/BP_MultiplayerSandbox_Projectile.BP_MultiplayerSandbox_Projectile_C" (`SceneComponent.K2_GetComponentToWorld` (`self.Arrow1`)) "AlwaysSpawn" "MultiplyWithRoot" self null))

(event `TakeDamage`
  (params (Damage :type "Float (double-precision)"))
  (bind _output_get (set `self.Health` (- (`self.Health`) Damage)))
  (if (<= _output_get 0.0)
    (`self.K2_DestroyActor`)))

(fn `UserConstructionScript`)